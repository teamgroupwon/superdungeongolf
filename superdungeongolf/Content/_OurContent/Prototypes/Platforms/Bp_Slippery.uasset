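; Slippery platform prototype that changes a ThirdPersonCharacter's movement while it overlaps the Box.
; BeginPlay caches the first player character's default ground friction and walking braking deceleration.
; Box overlap applies the sliding values to both properties on the entering character.
; Leaving restores the cached ground friction but sets braking deceleration to the sliding value again, so the cached braking default is never reapplied.
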(event `self.ReceiveBeginPlay`
  (bind _asthird_person_character (cast `/Game/ThirdPersonBP/Blueprints/ThirdPersonCharacter` (`GameplayStatics.GetPlayerCharacter` 0)))
  (bind _charactermovement (`Character.CharacterMovement` _asthird_person_character))
  (set `self.default ground friction` (`CharacterMovementComponent.GroundFriction` _charactermovement))
  (set `self.default braking friction` (`CharacterMovementComponent.BrakingDecelerationWalking` _charactermovement)))

(event `self.Box.OnComponentBeginOverlap`
  (params (OverlappedComponent :type "PrimitiveComponent Object Reference") (OtherActor :type "Actor Object Reference") (OtherComp :type "PrimitiveComponent Object Reference") (OtherBodyIndex :type Integer) (bFromSweep :type Boolean) (SweepResult :type "HitResult Structure (by ref)"))
  (bind _asthird_person_character (cast `/Game/ThirdPersonBP/Blueprints/ThirdPersonCharacter` OtherActor))
  (bind _charactermovement (`Character.CharacterMovement` _asthird_person_character))
  (set `CharacterMovementComponent.GroundFriction` (`self.sliding ground friction`) _charactermovement)
  (set `CharacterMovementComponent.BrakingDecelerationWalking` (`self.sliding brake friction`) _charactermovement))

(event `self.Box.OnComponentEndOverlap`
  (params (OverlappedComponent :type "PrimitiveComponent Object Reference") (OtherActor :type "Actor Object Reference") (OtherComp :type "PrimitiveComponent Object Reference") (OtherBodyIndex :type Integer))
  (bind _asthird_person_character (cast `/Game/ThirdPersonBP/Blueprints/ThirdPersonCharacter` OtherActor))
  (bind _charactermovement (`Character.CharacterMovement` _asthird_person_character))
  (set `CharacterMovementComponent.GroundFriction` (`self.default ground friction`) _charactermovement)
  (set `CharacterMovementComponent.BrakingDecelerationWalking` (`self.sliding brake friction`) _charactermovement))

(fn `UserConstructionScript`)