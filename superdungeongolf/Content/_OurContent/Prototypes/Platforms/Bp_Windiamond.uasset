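; Bp_Windiamond is a prototype goal trigger, apparently the win diamond that ends a timed run.
; When anything begins overlapping its Box, it changes the game manager's state and stops the timer, with no check on the overlapping actor.
; It then moves the manager's MyPlayer to just above the first PlayerStart found in the level, without sweep.
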(event `self.Box.OnComponentBeginOverlap`
  (params (OverlappedComponent :type "PrimitiveComponent Object Reference") (OtherActor :type "Actor Object Reference") (OtherComp :type "PrimitiveComponent Object Reference") (OtherBodyIndex :type Integer) (bFromSweep :type Boolean) (SweepResult :type "HitResult Structure (by ref)"))
  (bind _my_game_manager (`/Game/_OurContent/Blueprints/MyFunctionLibrary.Get My Game Manager`))
  (`/Game/_OurContent/Blueprints/MyGameManager.Set State` _my_game_manager "NewEnumerator1")
  (`/Game/_OurContent/Blueprints/MyGameManager.Stop Timer` _my_game_manager)
  (bind _outactors (`GameplayStatics.GetAllActorsOfClass` "/Script/Engine.PlayerStart"))
  (bind _my_game_manager_2 (`/Game/_OurContent/Blueprints/MyFunctionLibrary.Get My Game Manager`))
  (`self.K2_SetActorLocation` (`/Game/_OurContent/Blueprints/MyGameManager.My Player` _my_game_manager_2) (`KismetMathLibrary.MakeVector` (.x (`self.K2_GetActorLocation` (`|GetArrayItem` _outactors))) (.y (`self.K2_GetActorLocation` (`|GetArrayItem` _outactors))) (+ (.z (`self.K2_GetActorLocation` (`|GetArrayItem` _outactors))) 2.0)) false false))

(fn `UserConstructionScript`)