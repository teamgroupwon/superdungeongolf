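; Game manager actor that tracks the game state, Running or Abandon, and switches UI and mouse cursor to match.
; On BeginPlay it creates the abandon widget, adds it to the viewport and enters Running.
; SetState ignores unchanged states, otherwise hides the UI and applies the new state, with Abandon showing the widget and cursor.
; ResetGame moves the player to the first PlayerStart found.
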(event `self.ReceiveBeginPlay`
  (`self.Init`))

(fn `Create UI`
  (bind _returnvalue (`|CreateWidget` "/Game/_OurContent/Widgets/Widget_Abandon.Widget_Abandon_C"))
  (bind _output_get (set `self.Widget_Abandon` _returnvalue))
  (`UserWidget.AddToViewport` _output_get 0))

(fn `Get State`
  (returns (State :type Byte))
  (return (`self.Current Game State`)))

(fn `Init`
  (`self.Create UI`)
  (`self.Set State` "NewEnumerator0"))

(fn `Reset Game`
  (bind _outactors (`GameplayStatics.GetAllActorsOfClass` "/Script/Engine.PlayerStart"))
  (`self.K2_SetActorLocation` (`self.My Player`) (`self.K2_GetActorLocation` (`|GetArrayItem` _outactors)) false false))

(fn `Set State`
  (params (`New State` :type "/Game/_OurContent/Blueprints/MyGameStates Enum" :default "NewEnumerator0"))
  (if (`|EnumInequality` `New State` (`self.Current Game State`))
    (`/Game/_OurContent/Blueprints/MyFunctionLibrary.Hide UI`)
    (bind _output_get (set `self.Current Game State` `New State`))
    (switch `/Game/_OurContent/Blueprints/MyGameStates` _output_get
      (:`NewEnumerator0`
        (`/Game/_OurContent/Blueprints/MyFunctionLibrary.Show Mouse` false))
      (:`NewEnumerator3`
        (`Widget.SetVisibility` (`self.Widget_Abandon`) "Visible")
        (`/Game/_OurContent/Blueprints/MyFunctionLibrary.Show Mouse` true)))))

(fn `UserConstructionScript`)